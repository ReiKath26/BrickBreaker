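; Main_Player is the touch-controlled player for a ball game: it slides horizontally, launches balls and tracks lives.
; While touched, Tick traces under the first finger and moves the Player component to that X, keeping Y and pinning Z.
; A Ball spawns at the Arrow shortly after BeginPlay.
; Balls overlapping the Deadhe component cost a life, then either another spawns or the GameOver level opens when lives reach zero.
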(event OnComponentBeginOverlap(Deadhe)
  (params (OverlappedComponent :type Primitive%20Component%20Object%20Reference) (OtherActor :type Actor%20Object%20Reference) (OtherComp :type Primitive%20Component%20Object%20Reference) (OtherBodyIndex :type Integer) (bFromSweep :type Boolean) (SweepResult :type Hit%20Result%20Structure%20%28by%20ref%29))
  (bind _lifecount (Variables|Default|GetLifeCount))
  (Utilities|Casting|CastToBall OtherActor)
  (Math|Integer|DecrementInt _lifecount
    (:%20%20
      (if (== _lifecount 0)
        (Game|OpenLevel(byName) "GameOver")
        (else
          (Utilities|FlowControl|Delay 0.1)
          (Game|SpawnActorfromClass "/Game/Blueprint/Ball.Ball_C" (Transformation|GetWorldTransform (Variables|Default|GetArrow)) "Undefined" 0 0))))))

(event Custom|OnInputTouchBegin_Event
  (params (FingerIndex :type ETouchIndex%20Enum :default "Touch1") (TouchedActor :type Actor%20Object%20Reference)))

(event EventBeginPlay
  (bind _arrow (Variables|Default|GetArrow))
  (bind _returnvalue (Transformation|GetWorldLocation _arrow))
  (EventDispatchers|AssignOnInputTouchBegin (delegate Custom|OnInputTouchBegin_Event))
  (Transformation|SetWorldLocation _arrow (Math|Vector|MakeVector (.x _returnvalue) (.y _returnvalue) 1e+02) false false)
  (Utilities|FlowControl|Delay 1.0)
  (Game|SpawnActorfromClass "/Game/Blueprint/Ball.Ball_C" (Transformation|GetWorldTransform _arrow) "Undefined" 0 0))

(event Collision|EventActorBeginOverlap
  (params (OtherActor :type Actor%20Object%20Reference)))

(event EventTick
  (params (DeltaSeconds :type Float%20%28single-precision%29))
  (bind _player (Variables|Default|GetPlayer))
  (bind _player_2 (Variables|Default|GetPlayer))
  (if (Variables|Default|GetIsTouching)
    ;[1 1 1] if mouse is on screen
    (Transformation|SetWorldLocation _player (Math|Vector|MakeVector (.X (Math|Vector|BreakVector (.location (.HitResult (Class|PlayerController|GetHitResultUnderFingerbyChannel (Game|GetPlayerController 0) "Touch1" "TraceTypeQuery1" true))))) (.y (Transformation|GetWorldLocation _player)) 1e+02) false false)
    (else
      ;[1 1 1] if mouse is off screen
      (Transformation|SetWorldLocation _player_2 (Transformation|GetWorldLocation _player_2) false false))))

(event Input|TouchEvents|InputTouch
  (params (Location :type Vector) (FingerIndex :type ETouchIndex%20Enum))
  (:Pressed
    (Variables|Default|SetIsTouching true))
  (:Released
    (Variables|Default|SetIsTouching false)))

(fn ConstructionScript)