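; Brick actor that takes two Ball overlaps to destroy.
; The first Box overlap by a Ball swaps the Cube's material to MetalRed and sets a CanDestroy flag.
; A later overlap destroys the actor after a short delay.
; A Cube relocation node is present but unconnected, and the other events are empty.
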(event OnComponentBeginOverlap(Box)
  (params (OverlappedComponent :type Primitive%20Component%20Object%20Reference) (OtherActor :type Actor%20Object%20Reference) (OtherComp :type Primitive%20Component%20Object%20Reference) (OtherBodyIndex :type Integer) (bFromSweep :type Boolean) (SweepResult :type Hit%20Result%20Structure%20%28by%20ref%29))
  (Utilities|Casting|CastToBall OtherActor)
  (if (Variables|Default|GetCanDestroy)
    (Utilities|FlowControl|Delay 0.1)
    (Actor|DestroyActor)
    (else
      (Rendering|Material|SetMaterial (Variables|Default|GetCube) 0 "/Game/Material/MetalRed.MetalRed")
      (Variables|Default|SetCanDestroy true))))

(event EventBeginPlay)

(event Collision|EventActorBeginOverlap
  (params (OtherActor :type Actor%20Object%20Reference)))

(event EventTick
  (params (DeltaSeconds :type Float%20%28single-precision%29)))

(fn ConstructionScript)